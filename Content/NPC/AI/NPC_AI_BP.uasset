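; AI controller Blueprint for a guard NPC that reacts to the actors it perceives.
; On BeginPlay it initializes Patrol_Blackboard, caches the blackboard component and runs the Guard_Behavior tree.
; AI Perception updates write sensed actors lacking the "Enemy" tag into EnemyKey and clear the key when such an actor's stimulus is lost.
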(event `self.ReceiveBeginPlay`
  (bind _blackboardcomponent (`self.UseBlackboard` "/Game/NPC/AI/Patrol_Blackboard.Patrol_Blackboard"))
  (set `self.BlackbNPC` _blackboardcomponent)
  (`self.RunBehaviorTree` "/Game/NPC/AI/Guard_Behavior.Guard_Behavior"))

(event `self.ReceiveTick`
  (params (DeltaSeconds :type "Float (single-precision)")))

(event `self.AIPerception.OnTargetPerceptionUpdated`
  (params (Actor :type "Actor Object Reference") (Stimulus :type "AIStimulus Structure"))
  (if (`self.ActorHasTag` Actor "Enemy")
    _
    (elif (`.bSuccessfullySensed` (break `AIStimulus` Stimulus))
      (`BlackboardComponent.SetValueAsObject` (`self.BlackbNPC`) (`self.EnemyKey`) Actor)
      (else
        (`BlackboardComponent.ClearValue` (`self.BlackbNPC`) (`self.EnemyKey`))))))

(fn `UserConstructionScript`)